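; BP_EnemyPin is a marker actor that shows whether a shot at an enemy position was a hit or a miss.
; It holds two components, HitPin and MissedPin, both hidden with their children on BeginPlay.
; SetPinResult takes an IsHit flag and shows the matching pin while hiding the other.
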(event `self.ReceiveBeginPlay`
  (`SceneComponent.SetVisibility` (`self.MissedPin`) false true)
  (`SceneComponent.SetVisibility` (`self.HitPin`) false true))

(fn `SetPinResult`
  (params (bIsHit :type Boolean))
  (bind _hitpin (`self.HitPin`))
  (bind _missedpin (`self.MissedPin`))
  (if bIsHit
    (`SceneComponent.SetVisibility` _hitpin true true)
    (`SceneComponent.SetVisibility` _missedpin false true)
    (else
      (`SceneComponent.SetVisibility` _hitpin false true)
      (`SceneComponent.SetVisibility` _missedpin true true))))

(fn `UserConstructionScript`)